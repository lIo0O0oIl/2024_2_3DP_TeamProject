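; Interactive wardrobe for the CheapHotel environment whose two doors swing open and closed.
; Each Interaction event alternates through a FlipFlop between playing and reversing a Timeline, with an open or close sound at the actor's location.
; The Timeline's DoorFloat drives opposite yaw Lerps on the right and left doors, with the left Lerp also using DoorFloat as its start value.
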(event EventInteraction
  (bind _returnvalue (Transformation|GetActorLocation))
  (Utilities|FlowControl|FlipFlop
    (:A
      (Audio|PlaySoundatLocation "/Game/NeapolitanHotel/Sound/DoorOpen.DoorOpen" _returnvalue "0, 0, 0" 1.0 1.0 0.0 0 0 0 0)
      (bind _doorfloat (Timeline|Timeline Play)
        (:Update
          (Transformation|SetRelativeRotation (Variables|Default|GetS_Wardrobe_Door_R) (Math|Rotator|MakeRotator 0.0 0.0 (Math|Float|Lerp -1e+01 -1e+02 _doorfloat)) false false)
          (Transformation|SetRelativeRotation (Variables|Default|GetS_Wardrobe_Door_L) (Math|Rotator|MakeRotator 0.0 0.0 (Math|Float|Lerp _doorfloat 1e+02 _doorfloat)) false false))))
    (:B
      (Audio|PlaySoundatLocation "/Game/NeapolitanHotel/Sound/Door_Close.Door_Close" _returnvalue "0, 0, 0" 1.0 1.0 0.0 0 0 0 0)
      (Timeline|Timeline Reverse))))

(fn ConstructionScript)