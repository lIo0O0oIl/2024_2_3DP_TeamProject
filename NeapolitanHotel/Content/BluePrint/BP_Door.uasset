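; BP_Door is a door Blueprint that swings open and closed and can be locked.
; OpenDoor uses a FlipFlop to alternately play and reverse a timeline that lerps the Door component's yaw through a quarter turn, with open and close sounds.
; When IsLock is set, OpenDoor only plays the DoorUnlock sound.
; DoorLock toggles IsLock.
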(event Custom|OpenDoor
  (bind _self self)
  (bind _returnvalue (Transformation|GetActorLocation _self))
  (if (Variables|Default|GetIsLock)
    (Audio|PlaySoundatLocation "/Game/Sound/Door-Unlock.Door-Unlock" _returnvalue "0, 0, 0" 1.0 1.0 0.0 0 0 0 0)
    (else
      (Utilities|FlowControl|FlipFlop
        (:A
          (Audio|PlaySoundatLocation "/Game/Sound/Door_Open.Door_Open" _returnvalue "0, 0, 0" 1.0 1.0 0.0 0 0 0 0)
          (bind _doorfloat (Timeline|OpenDoorTimeLine Play)
            (:Update
              (Transformation|SetRelativeRotation (Variables|Default|GetDoor) (Math|Rotator|MakeRotator 0.0 0.0 (Math|Float|Lerp 0.0 9e+01 _doorfloat)) false false))))
        (:B
          (Audio|PlaySoundatLocation "/Game/Sound/Door_Close.Door_Close" _returnvalue "0, 0, 0" 1.0 1.0 0.0 0 0 0 0)
          (Timeline|OpenDoorTimeLine Reverse))))))

(event Custom|DoorLock
  (Variables|Default|SetIsLock (not (Variables|Default|GetIsLock))))

(fn ConstructionScript)