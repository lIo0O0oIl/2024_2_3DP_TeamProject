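; BP_CallOnMe is a phone actor that rings until it is answered.
; BeginPlay fires the Call event, which plays the PhoneAudio component.
; The Answer event stops the audio, hides the actor and disables collision on its Sphere and StaticMeshComponent.
; Nothing in this Blueprint triggers Answer itself.
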(event Custom|Answer
  (Audio|Components|Audio|Stop (Variables|Default|GetPhone_Audio))
  (Rendering|SetActorHiddenInGame true)
  (Collision|SetCollisionEnabled (Variables|Default|GetSphere) "NoCollision"))

(event Custom|Call
  (Audio|Components|Audio|Play (Variables|Default|GetPhone_Audio) 0.0))

(event EventBeginPlay
  (CallFunction|Call))

(fn ConstructionScript)