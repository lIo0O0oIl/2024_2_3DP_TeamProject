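; Security monitor actor that shows live feeds from linked security cameras on its screen.
; On BeginPlay it puts a dynamic material on the monitor and feeds it a render target from the first camera's scene capture, sized by viewport and camera quality.
; SwapCamera cycles through cameras, detaching the previous capture and creating a new render target each time.
; Player input events rotate the active camera, and a separate event toggles audio.
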(event Custom|SwapCamera
  (bind (_width _height) (CallFunction|GetWidthandHeight))
  (Variables|/Script/Engine.SceneCaptureComponent2D|SetTextureTarget (Variables|/Game/NeapolitanHotel/BluePrint/BP_SecurityCamera.BP_SecurityCamera_C|GetSceneCaptureComponent2D (Utilities|Array|Get(acopy) (Variables|Default|GetLinkedCameras) (Variables|Default|GetCurrentCamera))) 0)
  (Math|Integer|IncrementInt (Variables|Default|GetCurrentCamera)
    (:%20%20
      (if (>= (Variables|Default|GetCurrentCamera) (Utilities|Array|Length (Variables|Default|GetLinkedCameras)))
        (Variables|Default|SetCurrentCamera 0))
      (bind _returnvalue (Rendering|CreateRenderTarget2D _width _height "RTF_RGBA16f"))
      (bind _output_get (Variables|Default|SetRT_Camera _returnvalue))
      (bind _output_get_2 (Variables|/Script/Engine.SceneCaptureComponent2D|SetTextureTarget (Variables|/Game/NeapolitanHotel/BluePrint/BP_SecurityCamera.BP_SecurityCamera_C|GetSceneCaptureComponent2D (Utilities|Array|Get(acopy) (Variables|Default|GetLinkedCameras) (Variables|Default|GetCurrentCamera))) _output_get))
      (Rendering|Material|SetTextureParameterValue (Variables|Default|GetM_Camera) "Texture" _output_get_2))))

(event Custom|NewPlayerInput
  (params (HorizontalValue :type Float%20%28double-precision%29) (VerticalValue :type Float%20%28double-precision%29))
  (Default|RotateCamera (Utilities|Array|Get(acopy) (Variables|Default|GetLinkedCameras) (Variables|Default|GetCurrentCamera)) HorizontalValue VerticalValue))

(event Custom|Sound
  (bind _audio (Variables|Default|GetAudio))
  (Utilities|FlowControl|FlipFlop
    (:A
      (Audio|Components|Audio|Play _audio 0.0))
    (:B
      (Audio|Components|Audio|Stop _audio))))

(event EventBeginPlay
  (bind (_width _height) (CallFunction|GetWidthandHeight))
  (Utilities|IsValid (Utilities|Array|Get(acopy) (Variables|Default|GetLinkedCameras))
    (:Is%20Valid
      (bind _returnvalue (Rendering|Material|CreateDynamicMaterialInstance "/Game/NeapolitanHotel/Matrial/M_SecurityCamera.M_SecurityCamera" "None" "None" :!class /Script/Engine.KismetMaterialLibrary))
      (bind _output_get (Variables|Default|SetM_Camera _returnvalue))
      (Rendering|Material|SetMaterial (Variables|Default|GetMonitor) 0 _output_get)
      (bind _returnvalue_2 (Rendering|CreateRenderTarget2D _width _height "RTF_RGBA16f"))
      (bind _output_get_2 (Variables|Default|SetRT_Camera _returnvalue_2))
      (bind _output_get_3 (Variables|/Script/Engine.SceneCaptureComponent2D|SetTextureTarget (Variables|/Game/NeapolitanHotel/BluePrint/BP_SecurityCamera.BP_SecurityCamera_C|GetSceneCaptureComponent2D (Utilities|Array|Get(acopy) (Variables|Default|GetLinkedCameras))) _output_get_2))
      (Rendering|Material|SetTextureParameterValue (Variables|Default|GetM_Camera) "Texture" _output_get_3)
      (Rendering|Material|SetScalarParameterValue (Variables|Default|GetM_Camera) "ScreenBrightness" (Variables|Default|GetScreenBrightness) :!class /Script/Engine.MaterialInstanceDynamic))))

(fn ConstructionScript)

(fn GetWidthandHeight
  (bind _returnvalue (Viewport|GetViewportSize))
  (bind _linkedcameras (Variables|Default|GetLinkedCameras))
  (bind _currentcamera (Variables|Default|GetCurrentCamera))
  (bind _output (Utilities|Array|Get(acopy) _linkedcameras _currentcamera))
  (bind _cameraqualitylevel (Variables|/Game/NeapolitanHotel/BluePrint/BP_SecurityCamera.BP_SecurityCamera_C|GetCameraQualityLevel _output))
  (return (Math|Float|Truncate (* (.x _returnvalue) _cameraqualitylevel)) (Math|Float|Truncate (* (.y _returnvalue) _cameraqualitylevel))))