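; BP_Note is an interactable paper note that opens and closes a reading widget.
; Each Interaction plays a page-turn sound at the note, then a FlipFlop alternates between reading and putting it down.
; Reading adds a new UW_NoteWidget to the viewport, ignores player look and move input, and hides the Note component.
; Putting down calls NoteDown on the widget, restores input and shows the note again.
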(event EventInteraction
  (bind _returnvalue (Game|GetPlayerController 0))
  (bind _note (Variables|Default|GetNote))
  (Audio|PlaySoundatLocation "/Game/NeapolitanHotel/Sound/paperTurn.paperTurn" (Transformation|GetWorldLocation (Variables|Default|GetNote)) "0, 0, 0" 1.0 1.0 0.0 0 0 0 0)
  (Utilities|FlowControl|FlipFlop
    (:A
      (bind _returnvalue_2 (UserInterface|CreateWidget "/Game/NeapolitanHotel/UI/Game/UW_NoteWidget.UW_NoteWidget_C"))
      (UserInterface|Viewport|AddtoViewport _returnvalue_2 0)
      (Input|SetIgnoreLookInput _returnvalue true)
      (Input|SetIgnoreMoveInput _returnvalue true)
      (Rendering|SetVisibility _note false false))
    (:B
      (Default|NoteDown _returnvalue_2)
      (Input|SetIgnoreLookInput _returnvalue false)
      (Input|SetIgnoreMoveInput _returnvalue false)
      (Rendering|SetVisibility _note true false))))

(fn ConstructionScript)