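; BP_Telephone is a telephone gimmick that, while ringing, interferes with the lights.
; Interaction and GimmickStart share one FlipFlop that either starts the call sound and Call loop, or stops the sound and turns all lights back on.
; Call re-invokes itself on delays while IsCall is set, calling TurnOffTheLight each cycle.
; GameOver waits briefly, silences the phone and forwards game over to BP_GameManager.
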(event Custom|Call
  (Utilities|FlowControl|Delay 0.25)
  (Class|Telephone|TurnOfftheLight)
  (Utilities|FlowControl|Delay 2.7)
  (if (Variables|Default|GetIsCall)
    (CallFunction|Call)))

(event EventGimmickStart
  (bind _callsound (Variables|Default|GetCallSound))
  (Utilities|FlowControl|FlipFlop
    (:A
      (Audio|Components|Audio|Play _callsound 0.0)
      (CallFunction|Call)
      (Variables|Default|SetIsCall true))
    (:B
      (Audio|Components|Audio|Stop _callsound)
      (Class|Telephone|TurnontheAllLight)
      (Variables|Default|SetIsCall false))))

(event EventInteraction
  (bind _callsound (Variables|Default|GetCallSound))
  (Utilities|FlowControl|FlipFlop
    (:A
      (Audio|Components|Audio|Play _callsound 0.0)
      (CallFunction|Call)
      (Variables|Default|SetIsCall true))
    (:B
      (Audio|Components|Audio|Stop _callsound)
      (Class|Telephone|TurnontheAllLight)
      (Variables|Default|SetIsCall false))))

(event EventGameOver
  (Utilities|FlowControl|Delay 2.5)
  (Audio|Components|Audio|Stop (Variables|Default|GetCallSound))
  (bind _outactors (Actor|GetAllActorsOfClass "/Game/NeapolitanHotel/BluePrint/BP_GameManager.BP_GameManager_C"))
  (Default|GameOver (Utilities|Array|Get(acopy) _outactors)))

(fn ConstructionScript)