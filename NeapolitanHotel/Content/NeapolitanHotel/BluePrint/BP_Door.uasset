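; BP_Door is a hinged door Blueprint that swings open and closed and can be locked.
; OpenDoor alternates through a FlipFlop between playing and reversing a timeline that lerps the door's relative yaw up to a quarter turn.
; DoorLock toggles IsLock, which blocks only the opening branch, though a blocked call still advances the FlipFlop.
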(event Custom|OpenDoor
  (Utilities|FlowControl|FlipFlop
    (:A
      (if (not (Variables|Default|GetIsLock))
        (bind _doorfloat (Timeline|OpenDoorTimeLine Play)
          (:Update
            (Transformation|SetRelativeRotation (Variables|Default|GetDoor) (Math|Rotator|MakeRotator 0.0 0.0 (Math|Float|Lerp 0.0 9e+01 _doorfloat)) false false)))))
    (:B
      (Timeline|OpenDoorTimeLine Reverse))))

(event Custom|DoorLock
  (Variables|Default|SetIsLock (not (Variables|Default|GetIsLock))))

(fn ConstructionScript)