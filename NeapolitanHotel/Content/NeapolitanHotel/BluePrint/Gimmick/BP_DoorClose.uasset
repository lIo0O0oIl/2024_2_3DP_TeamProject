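; BP_DoorClose is a door gimmick that swings open when triggered and that an interaction shuts.
; GimmickStart clears IsLook, plays the open sound and runs a timeline that yaws the door between 0 and 90 degrees.
; Interaction reverses that timeline with a close sound and sets IsLook, after which further interactions only play the DoorUnlock sound.
; A separate GameOver event forwards to the first BP_GameManager found.
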(event EventGameOver
  (bind _outactors (Actor|GetAllActorsOfClass "/Game/NeapolitanHotel/BluePrint/BP_GameManager.BP_GameManager_C"))
  (Default|GameOver (Utilities|Array|Get(acopy) _outactors)))

(event EventInteraction
  (if (Variables|Default|GetIsLook)
    (Audio|PlaySoundatLocation "/Game/NeapolitanHotel/Sound/Door-Unlock.Door-Unlock" (Transformation|GetActorLocation) "0, 0, 0" 1.0 1.0 0.0 0 0 0 0)
    (else
      (Audio|PlaySoundatLocation "/Game/NeapolitanHotel/Sound/Door_Close.Door_Close" (Transformation|GetActorLocation) "0, 0, 0" 1.0 1.0 0.0 0 0 0 0)
      (Variables|Default|SetIsLook true)
      (bind _doorfloat (Timeline|Timeline Reverse)
        (:Update
          (Transformation|SetRelativeRotation (Variables|Default|GetS_Door_01_door) (Math|Rotator|MakeRotator 0.0 0.0 (Math|Float|Lerp 0.0 9e+01 _doorfloat)) false false))))))

(event EventGimmickStart
  (Variables|Default|SetIsLook false)
  (Audio|PlaySoundatLocation "/Game/NeapolitanHotel/Sound/DoorOpen.DoorOpen" (Transformation|GetActorLocation) "0, 0, 0" 1.0 1.0 0.0 0 0 0 0)
  (bind _doorfloat (Timeline|Timeline Play)
    (:Update
      (Transformation|SetRelativeRotation (Variables|Default|GetS_Door_01_door) (Math|Rotator|MakeRotator 0.0 0.0 (Math|Float|Lerp 0.0 9e+01 _doorfloat)) false false))))

(fn ConstructionScript)