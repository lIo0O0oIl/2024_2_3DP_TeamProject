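; BP_Telephone is a hotel gimmick: a ringing telephone that ends the game if the player interacts with it during the call.
; GimmickStart turns on all lights, plays the ring and starts a self-calling delayed loop that repeatedly calls TurnOffTheLight.
; GimmickClear clears IsCall, so the loop stops the sound on its next check.
; Interaction during a call, or the GameOver event, stops the ring after a delay and triggers GameOver on BP_GameManager.
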(event Custom|Call
  (Utilities|FlowControl|Delay 0.25)
  (Class|Telephone|TurnOfftheLight)
  (Utilities|FlowControl|Delay 2.7)
  (if (Variables|Default|GetIsCall)
    (CallFunction|Call)
    (else
      (Audio|Components|Audio|Stop (Variables|Default|GetCallSound)))))

(event EventGimmickStart
  (Class|Telephone|TurnontheAllLight)
  (Audio|Components|Audio|Play (Variables|Default|GetCallSound) 0.0)
  (CallFunction|Call)
  (Variables|Default|SetIsCall true))

(event EventInteraction
  (if (Variables|Default|GetIsCall)
    (Utilities|FlowControl|Delay 2.5)
    (Audio|Components|Audio|Stop (Variables|Default|GetCallSound))
    (bind _outactors (Actor|GetAllActorsOfClass "/Game/NeapolitanHotel/BluePrint/BP_GameManager.BP_GameManager_C"))
    (Default|GameOver (Utilities|Array|Get(acopy) _outactors))))

(event EventGameOver
  (Utilities|FlowControl|Delay 2.5)
  (Audio|Components|Audio|Stop (Variables|Default|GetCallSound))
  (bind _outactors (Actor|GetAllActorsOfClass "/Game/NeapolitanHotel/BluePrint/BP_GameManager.BP_GameManager_C"))
  (Default|GameOver (Utilities|Array|Get(acopy) _outactors)))

(event EventGimmickClear
  (Variables|Default|SetIsCall false))

(fn ConstructionScript)